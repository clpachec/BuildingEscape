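; Openable door actor that swings open and closed when its OpenDoor component or interface fires open and close events.
; BeginPlay caches the initial rotation, and the DoorAnimation timeline drives a yaw offset combined with it.
; Opening plays the timeline, with an event track playing the Door_Lock sound at the door's location; closing reverses it.
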(event `self.ReceiveBeginPlay`
  (set `self.Initial Rotation` (`self.K2_GetActorRotation`)))

(event `self.OpenDoor.OnOpen`
  (bind (_direction _open_door) (`Timeline|Door Animation` :!label _label)
    (:`Update`
      (`self.K2_SetActorRotation` (`KismetMathLibrary.ComposeRotators` (`KismetMathLibrary.MakeRotator` 0.0 0.0 _open_door) (`self.Initial Rotation`))))
    (:`SFX Door Opening`
      (`GameplayStatics.PlaySoundAtLocation` "/Game/Audio/Door_Lock.Door_Lock" (`self.K2_GetActorLocation`)))))

(event `self.OpenDoor.OnClose`
  (goto _label :!via `Reverse`))

(fn `UserConstructionScript`)